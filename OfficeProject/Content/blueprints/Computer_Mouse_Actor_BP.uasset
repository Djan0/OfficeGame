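; Computer mouse actor that moves with horizontal mouse input, apparently an early prototype of an in-world mouse or cursor.
; Mouse X offsets the actor's location equally along world X and Z without sweeping, unless Left Alt is held; Mouse Y is unused.
; Left click only prints a debug greeting when ClickableObject is valid, and nothing in these graphs assigns that variable.
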(event EventBeginPlay)

(event Collision|EventActorBeginOverlap
  (params (OtherActor :type Actor%20Object%20Reference)))

(event EventTick
  (params (DeltaSeconds :type Float%20%28single-precision%29)))

(event Input|MouseEvents|MouseY
  (params (AxisValue :type Float%20%28single-precision%29)))

(event Input|MouseEvents|MouseX
  (params (AxisValue :type Float%20%28single-precision%29))
  (if (not (Variables|Default|GetAltPressed))
    (Transformation|SetActorLocation (+ (Math|Vector|MakeVector AxisValue 0.0 (stale Input|MouseEvents|MouseY AxisValue)) (Transformation|GetActorLocation)) false false)))

(event Input|KeyboardEvents|LeftAlt
  (params (Key :type Key%20Structure))
  (:Pressed
    (Variables|Default|SetAltPressed true))
  (:Released
    (Variables|Default|SetAltPressed false)))

(event Input|MouseEvents|LeftMouseButton
  (params (Key :type Key%20Structure))
  (:Pressed
    (Utilities|IsValid (Variables|Default|GetClickableObject)
      (:Is%20Valid
        (Development|PrintString "Hello")))))

(fn ConstructionScript)